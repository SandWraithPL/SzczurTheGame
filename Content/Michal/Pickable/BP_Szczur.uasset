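; BP_Szczur is a rat ("szczur") pawn that wanders in random directions.
; A looping timer, with its interval randomized at BeginPlay, rerolls two direction values that Tick feeds into movement input.
; Tick also mirrors the Szczur component through negative X scale according to the Y direction's sign.
; An alternative AIMoveTo event targeting random points exists, but its timer is never run.
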(event Custom|AI_Ruchu
  (AI|AIMoveTo 0 (Math|Vector|MakeVector (Math|Random|RandomFloatinRange 3.3e+02 1.23e+03) (Math|Random|RandomFloatinRange -1.29e+03 -3.9e+02) 0.0) 0 5.0 false
    (:then
      (Development|PrintString "ruch"))))

(event Custom|Losuj%20kierunki
  (Variables|Default|Setkierunek1 (Math|Random|RandomFloatinRange -1.0 1.0))
  (Variables|Default|Setkierunek2 (Math|Random|RandomFloatinRange -1.0 1.0)))

(event Custom|CustomEvent12)

(event EventTick
  (params (DeltaSeconds :type Float%20%28single-precision%29))
  (bind _kierunek2 (Variables|Default|Getkierunek2))
  (Pawn|Input|AddMovementInput (Math|Vector|MakeVector (Variables|Default|Getkierunek1) _kierunek2 0.0) 1e+02 false)
  (if (> _kierunek2 0.0)
    (Transformation|SetWorldScale3D (Variables|Default|Get%20szczur) "10.500000,1.000000,10.500000")
    (else
      (Transformation|SetWorldScale3D (Variables|Default|Get%20szczur) "-10.500000,1.000000,10.500000"))))

(event EventBeginPlay
  (Variables|Default|Setkierunek1 (Math|Random|RandomFloatinRange -1.0 1.0))
  (Variables|Default|Setkierunek2 (Math|Random|RandomFloatinRange -1.0 1.0))
  (Utilities|Time|SetTimerbyEvent (delegate Custom|Losuj%20kierunki) (Math|Random|RandomFloatinRange 0.8 2.0) true))

(fn ConstructionScript)